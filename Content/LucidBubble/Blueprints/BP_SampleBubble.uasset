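; BP_SampleBubble is a bubble actor that can be launched as a physics projectile.
; BeginPlay runs the parent logic, then applies the Material variable to the first slot of its static mesh.
; Fire enables physics simulation on the mesh and replaces its linear velocity with the mesh's forward vector scaled by NewVelocity.
; Overlap, Tick and the construction script are empty.
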(event EventBeginPlay
  (|CallParentFunction)
  (Rendering|Material|SetMaterial (Variables|Default|GetStaticMesh) 0 (Variables|Default|GetMaterial)))

(event Collision|EventActorBeginOverlap
  (params (OtherActor :type Actor%20Object%20Reference)))

(event EventTick
  (params (DeltaSeconds :type Float%20%28single-precision%29)))

(fn ConstructionScript)

(fn Fire
  (params (NewVelocity :type Float%20%28single-precision%29))
  (Physics|SetSimulatePhysics (Variables|Default|GetStaticMesh) true)
  (Physics|SetPhysicsLinearVelocity (Variables|Default|GetStaticMesh) (* (Math|Vector|GetForwardVector (Transformation|GetWorldRotation (Variables|Default|GetStaticMesh))) NewVelocity) false "None"))